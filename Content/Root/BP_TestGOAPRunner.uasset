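; BP_TestGOAPRunner is a test Blueprint that smoke-tests the GOAP planner when play begins.
; It asks GOAPPlanner to build a plan from an unloaded-weapon world state to a loaded-weapon goal, offering the test reload action as the only available action.
; It prints the first planned action's name in green, or a red Russian "plan not found" message on failure, without executing the plan.
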(event `self.ReceiveBeginPlay`
  (bind (_outplan _returnvalue) (`GOAPPlannerComponent.BuildPlan` (`self.GOAPPlanner`) (`|MakeMap` (struct :`TagName` "World.WeaponLoaded") :!type "GameplayTag Structure") (`|MakeMap` (struct :`TagName` "World.WeaponLoaded") true :!type "GameplayTag Structure") (`|MakeArray` "/Game/Root/DA_Action_TestReload.DA_Action_TestReload" :!type "GOAPAction Object Reference")))
  (if _returnvalue
    (`KismetSystemLibrary.PrintString` (`KismetStringLibrary.Conv_NameToString` (`GOAPAction.ActionName` (`|GetArrayItem` _outplan))) true true (struct :`R` 0.011539 :`G` 1.0 :`B` 0.198197 :`A` 1.0))
    (else
      (`KismetSystemLibrary.PrintString` (`KismetStringLibrary.Concat_StrStr` "План не найден!") true true (struct :`R` 1.0 :`B` 0.082112 :`A` 1.0)))))

(fn `UserConstructionScript`)