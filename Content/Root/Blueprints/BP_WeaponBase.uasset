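; Base first-person weapon actor that handles equipping, automatic hitscan fire and reloading, driven by a WeaponConfig asset.
; A looping fire-rate timer calls PerformShot, which spends ammo, traces a random spread cone from the owner's camera, adds recoil and shake, and applies damage.
; Reload picks empty or tactical montages, waits out the hands montage, then refills from reserve.
; A shared helper plays paired arms and weapon montages; fire and reload montages are hard-coded, mostly PKM.
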(event `self.ReceiveBeginPlay`
  ; сетаем боезапас из конфига
  (set `self.CurrentAmmo` (`/Game/Root/DataAssets/PDA_WeaponConfig.MagCapacity` (`self.WeaponConfig`)))
  (set `self.CurrentReserveAmmo` (`/Game/Root/DataAssets/PDA_WeaponConfig.MaxAmmoCap` (`self.WeaponConfig`))))

(event `OnEquip`
  ; Вызов монтажа Draw при подборе оружия
  (`self.PlayWeaponMontages` (`/Game/Root/DataAssets/PDA_WeaponConfig.Montage_Draw_Hands` (`self.WeaponConfig`)) (`/Game/Root/DataAssets/PDA_WeaponConfig.Montage_Draw_Weapon` (`self.WeaponConfig`))))

(event `StartFIre`
  ; Запуск и остановка стрельбы
  (if (not (`self.bIsReloading`))
    (`self.PerformShot`)
    (bind _returnvalue (`KismetSystemLibrary.K2_SetTimerDelegate` (delegate `PerformShot`) (/ 60.0 (`/Game/Root/DataAssets/PDA_WeaponConfig.FireRate` (`self.WeaponConfig`))) true))
    (set `self.FireTimer` _returnvalue)))

(event `StopFire`
  ; Запуск и остановка стрельбы
  (`KismetSystemLibrary.K2_ClearAndInvalidateTimerHandle` (`self.FireTimer`)))

(event `PerformShot`
  ; Ивент на выстрел + проигрываем монтаж выстрела для рук и оружия
  (if (and (> (`self.CurrentAmmo`) 0) (not (`self.bIsReloading`)))
    ;; Вычитаем 1 патрон
    (`/Engine/EditorBlueprintResources/StandardMacros.DecrementInt` (`self.CurrentAmmo`)
      (:`  `
        (`self.PlayWeaponMontages` "/Game/Root/Assets/Anims/Montages/AM_Fire_Hands_sh.AM_Fire_Hands_sh" "/Game/Root/Assets/Anims/Montages/AM_Fire_PKM_Sh.AM_Fire_PKM_Sh")
        (`KismetSystemLibrary.PrintString` (`KismetStringLibrary.Conv_IntToString` (`self.CurrentAmmo`)) true false (struct :`R` 1.0 :`G` 0.081104 :`B` 0.073465 :`A` 1.0))
        (bind _asbp_player_character (cast `/Game/Root/Blueprints/BP_PlayerCharacter` (`self.GetOwner`)))
        (set `self.PlayerChar` _asbp_player_character)
        (bind _fpscamera (`/Game/Root/Blueprints/BP_PlayerCharacter.FPSCamera` _asbp_player_character))
        (bind (_outhit _returnvalue) (`KismetSystemLibrary.LineTraceSingle` (`SceneComponent.K2_GetComponentLocation` (`/Game/Root/Blueprints/BP_PlayerCharacter.FPSCamera` _asbp_player_character)) (+ (`SceneComponent.K2_GetComponentLocation` _fpscamera) (* (`KismetMathLibrary.RandomUnitVectorInConeInDegrees` (`SceneComponent.GetForwardVector` _fpscamera) (`/Game/Root/DataAssets/PDA_WeaponConfig.HipSpreadAngle` (`self.WeaponConfig`))) (`/Game/Root/DataAssets/PDA_WeaponConfig.MaxRange` (`self.WeaponConfig`)))) "TraceTypeQuery1" false (`|MakeArray` self (`self.GetOwner`) :!type "Actor Object Reference") "ForDuration"))
        ;; Добавление отдачи
        (`Pawn.AddControllerPitchInput` (`self.PlayerChar`) (`/Game/Root/DataAssets/PDA_WeaponConfig.VerticalRecoil` (`self.WeaponConfig`)))
        (`Pawn.AddControllerYawInput` (`self.PlayerChar`) (`/Game/Root/DataAssets/PDA_WeaponConfig.HorizontalRecoil` (`self.WeaponConfig`)))
        (`PlayerCameraManager.StartCameraShake` :`self` (`GameplayStatics.GetPlayerCameraManager` 0) :`ShakeClass` (`/Game/Root/DataAssets/PDA_WeaponConfig.FireCameraShake` (`self.WeaponConfig`)))
        (if _returnvalue
          (`GameplayStatics.ApplyDamage` (`.HitActor` (`GameplayStatics.BreakHitResult` _outhit)) (`/Game/Root/DataAssets/PDA_WeaponConfig.BaseDamage` (`self.WeaponConfig`)) (`self.GetInstigatorController` (`self.GetOwner`)) self))))
    (else
      (`self.StopFire`))))

(event `StartReload`
  ; Проверяем условия и запускаем монтаж перезарядки - тактической или полной
  (if (and (not (`self.bIsReloading`)) (< (`self.CurrentAmmo`) (`/Game/Root/DataAssets/PDA_WeaponConfig.MagCapacity` (`self.WeaponConfig`))) (> (`self.CurrentReserveAmmo`) 0))
    (`self.StopFire`)
    (set `self.bIsReloading` true)
    (if (== (`self.CurrentAmmo`) 0)
      (bind _duration (`self.PlayWeaponMontages` "/Game/Root/Assets/Anims/Montages/AM_Hands_Reload_Empty.AM_Hands_Reload_Empty" "/Game/Root/Assets/Anims/Montages/AM_PKM_Reload_Empty.AM_PKM_Reload_Empty"))
      (`KismetSystemLibrary.Delay` _duration)
      (else
        (bind _duration_2 (`self.PlayWeaponMontages` "/Game/Root/Assets/Anims/Montages/AM_Hands_Reload.AM_Hands_Reload" "/Game/Root/Assets/Anims/Montages/AM_PKM_Reload.AM_PKM_Reload"))
        (`KismetSystemLibrary.Delay` _duration_2)))
    ;; Обновляем кол-во патронов + снимаем статус перезарядки
    (set `self.AmmoToReload` (`KismetMathLibrary.Min` (- (`/Game/Root/DataAssets/PDA_WeaponConfig.MagCapacity` (`self.WeaponConfig`)) (`self.CurrentAmmo`)) (`self.CurrentReserveAmmo`)))
    (set `self.CurrentAmmo` (+ (`self.CurrentAmmo`) (`self.AmmoToReload`)))
    (set `self.CurrentReserveAmmo` (- (`self.CurrentReserveAmmo`) (`self.AmmoToReload`)))
    (set `self.bIsReloading` false)))

(fn `PlayWeaponMontages`
  (params (HandsMontage :type "AnimMontage Object Reference") (WeaponMontage :type "AnimMontage Object Reference"))
  (returns (Duration :type "Float (double-precision)"))
  ; Функция с помощью которой мы передаем монтажи, она вызывается  в Event Graph, логика повторяющаяся, поэтому вынесена в функцию
  (`AnimInstance.Montage_Play` (`SkeletalMeshComponent.GetAnimInstance` (`self.WeaponComponent`)) WeaponMontage 1.0 "MontageLength" 0.0 true)
  (bind _asbp_player_character (cast `/Game/Root/Blueprints/BP_PlayerCharacter` (`self.GetOwner`)))
  (bind _returnvalue (`AnimInstance.Montage_Play` (`SkeletalMeshComponent.GetAnimInstance` (`/Game/Root/Blueprints/BP_PlayerCharacter.FPS_Arms` _asbp_player_character)) HandsMontage 1.0 "MontageLength" 0.0 true))
  (return _returnvalue))

(fn `UserConstructionScript`
  (bind _weaponconfig (`self.WeaponConfig`)
    (:`then`
      (set `SkeletalMeshComponent.SkeletalMeshAsset` (`/Game/Root/DataAssets/PDA_WeaponConfig.WeaponMesh` _weaponconfig) (`self.WeaponComponent`)))
    (:`else`)))