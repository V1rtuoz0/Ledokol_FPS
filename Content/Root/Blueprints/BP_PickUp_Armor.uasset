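; Armor pickup actor that restores the player character's armor when stepped on.
; When the PickUpZone overlaps a BP_PlayerCharacter whose armor is below its maximum, it adds a fixed amount to CurrentArmor and destroys itself.
; The new value is clamped to a hardcoded range rather than to the character's MaxArmor, and the pickup stays in place if armor is already full.
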(event `self.PickUp Zone.OnComponentBeginOverlap`
  (params (OverlappedComponent :type "PrimitiveComponent Object Reference") (OtherActor :type "Actor Object Reference") (OtherComp :type "PrimitiveComponent Object Reference") (OtherBodyIndex :type Integer) (bFromSweep :type Boolean) (SweepResult :type "HitResult Structure (by ref)"))
  ; Прибавляем армор наступая на планку, удаляем его при подборе
  (bind _asbp_player_character (cast `/Game/Root/Blueprints/BP_PlayerCharacter` OtherActor))
  (set `self.PlayerRef` _asbp_player_character)
  (if (< (`/Game/Root/Blueprints/BP_PlayerCharacter.CurrentArmor` (`self.PlayerRef`)) (`/Game/Root/Blueprints/BP_PlayerCharacter.MaxArmor` (`self.PlayerRef`)))
    (set `/Game/Root/Blueprints/BP_PlayerCharacter.CurrentArmor` (`KismetMathLibrary.FClamp` (+ (`/Game/Root/Blueprints/BP_PlayerCharacter.CurrentArmor` (`self.PlayerRef`)) 20.0) 0.0 100.0) (`self.PlayerRef`))
    (`self.K2_DestroyActor`)))

(fn `UserConstructionScript`)